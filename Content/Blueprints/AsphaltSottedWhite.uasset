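; AsphaltSottedWhite is a spline-placed actor, likely a white asphalt road marking judging by its name.
; The construction script adds a spline mesh component for each segment between consecutive spline points, attached to the root and bent using local positions and tangents.
; Each piece is rolled on its side and given a narrow fixed scale, which is also applied to the spline itself.
; The event graph holds no active logic.
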(fn `UserConstructionScript`
  (bind _spline (`self.Spline`))
  (bind _spline_2 (`self.Spline`))
  (for _index (range (+ (- (`SplineComponent.GetNumberOfSplinePoints` _spline_2) 2) 1))
    (bind _returnvalue (`AddComponent|NODE_AddSplineMeshComponent-0`))
    (`SceneComponent.SetWorldScale3D` _returnvalue (0.05 0.5 0.5))
    (`SceneComponent.K2_SetWorldRotation` _returnvalue (`KismetMathLibrary.MakeRotator` -90.0 (.pitch (`SceneComponent.K2_GetComponentRotation` _returnvalue)) (.yaw (`SceneComponent.K2_GetComponentRotation` _returnvalue))) false false)
    (`SceneComponent.K2_AttachToComponent` _returnvalue (`self.DefaultSceneRoot`) "None" "KeepRelative" "KeepRelative" "KeepRelative" true)
    (bind (_location _tangent) (`SplineComponent.GetLocationAndTangentAtSplinePoint` _spline _index "Local"))
    (bind (_location_2 _tangent_2) (`SplineComponent.GetLocationAndTangentAtSplinePoint` _spline (+ _index 1) "Local"))
    (`SplineMeshComponent.SetStartAndEnd` _returnvalue _location _tangent _location_2 _tangent_2 true)
    (`SceneComponent.SetWorldScale3D` _spline_2 (0.05 0.5 0.5))))